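; BP_Demo is a demo Blueprint that bootstraps the root UI and handles the pause menu input.
; On BeginPlay it creates a UI_RootLayout widget for the first player, adds it to the viewport and sets its initial MenuState.
; Escape and Gamepad Special Right share one gated path that switches MenuState to open the pause menu, conditioned on the current menu state.
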(event `self.ReceiveBeginPlay`
  (bind _rootwidget (`self.RootWidget`))
  (`|ExecutionSequence`
    (:`then_0`
      (bind _returnvalue (`|CreateWidget` "/Game/UI/UI_RootLayout.UI_RootLayout_C" (`GameplayStatics.GetPlayerController` 0)))
      (set `self.RootWidget` _returnvalue))
    (:`then_1`
      (`UserWidget.AddToViewport` _rootwidget 0))
    (:`then_2`
      (set `/Game/UI/UI_RootLayout.MenuState` "NewEnumerator1" _rootwidget))))

(event `Key|Escape`
  (params (Key :type "Key Structure"))
  (bind _rootwidget (`self.RootWidget`))
  (:`Pressed`
    (`/Engine/EditorBlueprintResources/StandardMacros.Gate` (not (`|EnumEquality` (`/Game/UI/UI_RootLayout.MenuState` _rootwidget) "NewEnumerator2")) :!label _label
      (:`Exit`
        (set `/Game/UI/UI_RootLayout.MenuState` "NewEnumerator8" _rootwidget)))))

(event `Key|Gamepad_Special_Right`
  (params (Key :type "Key Structure"))
  (:`Pressed`
    (goto _label)))

(fn `UserConstructionScript`)